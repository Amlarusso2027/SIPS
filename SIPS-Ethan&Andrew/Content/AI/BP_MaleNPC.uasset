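; Male NPC that tracks its proximity to BP_Boby and plays multi-line dialogue.
; Each tick it toggles the AI blackboard flag hasSeenBoby by distance, using separate enter and exit thresholds for hysteresis.
; The Talk event steps through the Dialogue array in a WBP_Dialogue widget, created if none is valid, otherwise reused with its CurrentIndex reset.
; After the last line it resets the index and removes the widget.
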(event `self.ReceiveTick`
  (params (DeltaSeconds :type "Float (single-precision)"))
  (bind _returnvalue (`AIBlueprintHelperLibrary.GetBlackboard` (`AIBlueprintHelperLibrary.GetAIController` self)))
  (bind _returnvalue_2 (`GameplayStatics.GetActorOfClass` "/Game/AI/BP_Boby.BP_Boby_C"))
  (`/Engine/EditorBlueprintResources/StandardMacros.IsValid` _returnvalue_2
    (:`Is Valid`
      (if (`BlackboardComponent.GetValueAsBool` _returnvalue "hasSeenBoby")
        (bind _returnvalue_3 (`self.GetDistanceTo` _returnvalue_2 self))
        (if (> _returnvalue_3 1500.0)
          (`BlackboardComponent.SetValueAsBool` _returnvalue "hasSeenBoby" false))
        (elif (< _returnvalue_3 1000.0)
          (`BlackboardComponent.SetValueAsBool` _returnvalue "hasSeenBoby" true))))))

(event `/Game/Dialogue/BPI_Dialogue.Talk`
  (`/Engine/EditorBlueprintResources/StandardMacros.IncrementInt` (`self.TalkIndex`)
    (:`  `
      (if (< (`self.TalkIndex`) (`KismetArrayLibrary.Array_Length` (`self.Dialogue`)))
        (`self.UI`
          (:`then`
            (set `/Game/Dialogue/WBP_Dialogue.CurrentIndex` 0 (`self.UI`)))
          (:`else`
            (bind _returnvalue (`|CreateWidget` "/Game/Dialogue/WBP_Dialogue.WBP_Dialogue_C" (`GameplayStatics.GetPlayerController` 0)))
            (bind _output_get (set `self.UI` _returnvalue))
            (`UserWidget.AddToViewport` _output_get 0)))
        (set `/Game/Dialogue/WBP_Dialogue.FullText` (`|GetArrayItem` (`self.Dialogue`) (`self.TalkIndex`)) (`self.UI`))
        (else
          (set `self.TalkIndex` -1)
          (`Widget.RemoveFromParent` (`self.UI`)))))))

(fn `UserConstructionScript`)