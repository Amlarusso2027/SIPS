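; Interactable wiring puzzle station that, once enabled, is marked broken and offers a repair prompt.
; A 15-second neglect timer then messages every Wiring_neglect actor and prints a power warning.
; Interacting opens WBP_WiringBoard, switching to UI-only input and flagging the player's BPC_Interactor as in a minigame.
; Solving prints success and closes the board after a delay, and closing restores game input, but nothing here clears Broken or the timer.
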(event `self.wiring_enable`
  (set `self.broken` true)
  (`KismetSystemLibrary.K2_SetTimerDelegate` (delegate `wiring neglected`) 15.0))

(event `wiring neglected`
  (bind _outactors (`GameplayStatics.GetAllActorsWithInterface` "/Game/Puzzle/Wiring/wiring_neglect.wiring_neglect_C"))
  (message `/Game/Puzzle/Wiring/wiring_neglect.wiring_neglect` _outactors)
  (`KismetSystemLibrary.PrintString` "Warning: power fluctuations compromising bunker systems"))

(event `self.Interact`
  (params (Interactor :type "Actor Object Reference"))
  (bind _returnvalue (`GameplayStatics.GetPlayerController` 0))
  (set `/Game/Puzzle/Blueprints/Interaction/BPC_Interactor.bInMinigame` true (`self.GetComponentByClass` (`GameplayStatics.GetPlayerPawn` 0) "/Game/Puzzle/Blueprints/Interaction/BPC_Interactor.BPC_Interactor_C"))
  (bind _returnvalue_2 (`|CreateWidget` "/Game/Puzzle/Wiring/WBP_WiringBoard.WBP_WiringBoard_C" (`GameplayStatics.GetPlayerController` 0)))
  (`|ExecutionSequence`
    (:`then_0`
      (`UserWidget.AddToViewport` _returnvalue_2 0))
    (:`then_1`
      (add `/Game/Puzzle/Wiring/WBP_WiringBoard.OnBoardClosed` _returnvalue_2 (delegate `HandleBoardClosed`))
      (`WidgetBlueprintLibrary.SetInputMode_UIOnlyEx` _returnvalue _returnvalue_2))
    (:`then_2`
      (set `PlayerController.bShowMouseCursor` true _returnvalue))
    (:`then_3`
      (set `self.BoardWidget` _returnvalue_2)
      (add `/Game/Puzzle/Wiring/WBP_WiringBoard.OnBoardSolved` _returnvalue_2 (delegate `HandleBoardSolved`)))))

(event `HandleBoardClosed`
  (bind _returnvalue (`GameplayStatics.GetPlayerController` 0))
  (`|ExecutionSequence`
    (:`then_0`
      (`WidgetBlueprintLibrary.SetInputMode_GameOnly` _returnvalue))
    (:`then_1`
      (set `PlayerController.bShowMouseCursor` false _returnvalue)
      (set `/Game/Puzzle/Blueprints/Interaction/BPC_Interactor.bInMinigame` false (`self.GetComponentByClass` (`GameplayStatics.GetPlayerPawn` 0) "/Game/Puzzle/Blueprints/Interaction/BPC_Interactor.BPC_Interactor_C")))))

(event `HandleBoardSolved`
  (bind _boardwidget (`self.BoardWidget`))
  (`KismetSystemLibrary.PrintString` "Life support restored!")
  (`KismetSystemLibrary.Delay` 1.5)
  (`/Engine/EditorBlueprintResources/StandardMacros.IsValid` _boardwidget
    (:`Is Valid`
      (`/Game/Puzzle/Wiring/WBP_WiringBoard.CloseBoard` _boardwidget))))

(fn `GetPromptText`
  (returns (Prompt :type Text))
  (if (`self.broken`)
    (return "Press E to repair wiring")
    (else
      (return "System functional"))))

(fn `UserConstructionScript`)