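; BP_FoodSynthesizer is an interactable food synthesizer puzzle that can break and be recalibrated through a quick-time-event minigame.
; FSEnable sets it broken and starts a timer that broadcasts a neglect message to all FS_neglect interface actors.
; Interacting while broken opens WBP_FoodSynthQTE in UI-only input and flags the player's interactor as in a minigame.
; The finish callback restores game input and prints the result, leaving Broken and the timer untouched.
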(event `self.FS_enable`
  (set `self.broken` true)
  (`KismetSystemLibrary.K2_SetTimerDelegate` (delegate `FS neglected`) 10.0))

(event `FS neglected`
  (bind _outactors (`GameplayStatics.GetAllActorsWithInterface` "/Game/Puzzle/FoodSynth/FS_neglect.FS_neglect_C"))
  (message `/Game/Puzzle/FoodSynth/FS_neglect.FS_neglect` _outactors)
  (`KismetSystemLibrary.PrintString` "Error: food synthesizer print failure"))

(event `self.Interact`
  (params (Interactor :type "Actor Object Reference"))
  (bind _returnvalue (`GameplayStatics.GetPlayerController` 0))
  (if (`self.broken`)
    (if (not (`self.bInUse`))
      (set `self.bInUse` true)
      (set `/Game/Puzzle/Blueprints/Interaction/BPC_Interactor.bInMinigame` true (`self.GetComponentByClass` (`GameplayStatics.GetPlayerPawn` 0) "/Game/Puzzle/Blueprints/Interaction/BPC_Interactor.BPC_Interactor_C"))
      (bind _returnvalue_2 (`|CreateWidget` "/Game/Puzzle/FoodSynth/WBP_FoodSynthQTE.WBP_FoodSynthQTE_C" (`GameplayStatics.GetPlayerController` 0)))
      (`|ExecutionSequence`
        (:`then_0`
          (`UserWidget.AddToViewport` _returnvalue_2 0))
        (:`then_1`
          (add `/Game/Puzzle/FoodSynth/WBP_FoodSynthQTE.OnQTEFinished` _returnvalue_2 (delegate `HandleQTEFinished`))
          (`WidgetBlueprintLibrary.SetInputMode_UIOnlyEx` _returnvalue _returnvalue_2))
        (:`then_2`
          (set `PlayerController.bShowMouseCursor` true _returnvalue))))))

(event `HandleQTEFinished`
  (params (Success :type Boolean))
  (bind _returnvalue (`GameplayStatics.GetPlayerController` 0))
  (`|ExecutionSequence`
    (:`then_0`
      (`WidgetBlueprintLibrary.SetInputMode_GameOnly` _returnvalue))
    (:`then_1`
      (set `PlayerController.bShowMouseCursor` false _returnvalue)
      (set `self.bInUse` false)
      (set `/Game/Puzzle/Blueprints/Interaction/BPC_Interactor.bInMinigame` false (`self.GetComponentByClass` (`GameplayStatics.GetPlayerPawn` 0) "/Game/Puzzle/Blueprints/Interaction/BPC_Interactor.BPC_Interactor_C"))
      (if Success
        (`KismetSystemLibrary.PrintString` "Food Printed!")
        (else
          (`KismetSystemLibrary.PrintString` "Metallic goop everywhere..."))))))

(fn `GetPromptText`
  (returns (Prompt :type Text))
  (if (`self.broken`)
    (return "Press E to recalibrate")
    (else
      (return "System functional"))))

(fn `UserConstructionScript`)