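; Player interaction component that finds interactable actors in view and triggers them on the Interact input.
; A short sphere trace along the third-person follow camera, starting just past the boom arm length, returns hit actors implementing BPI_Interactable.
; Tick shows that actor's prompt text in a widget created at BeginPlay, hiding it during minigames or when nothing is found.
; IA_Interact repeats the trace and sends InteractMessage to the target with the owner.
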(event `self.ReceiveBeginPlay`
  (bind _returnvalue (`|CreateWidget` "/Game/Puzzle/UI/WBP_InteractPrompt.WBP_InteractPrompt_C" (`GameplayStatics.GetPlayerController` 0)))
  (bind _output_get (set `self.PromptWidget` _returnvalue))
  (`UserWidget.AddToViewport` _output_get 0)
  (`Widget.SetVisibility` _output_get "Hidden"))

(event `self.ReceiveTick`
  (params (DeltaSeconds :type "Float (single-precision)"))
  (if (`self.bInMinigame`)
    (`Widget.SetVisibility` (`self.PromptWidget`) "Hidden")
    (else
      (bind _hitactor (`self.GetLookedAtInteractable`))
      (`/Engine/EditorBlueprintResources/StandardMacros.IsValid` _hitactor
        (:`Is Valid`
          (bind _prompt (message `/Game/Puzzle/Blueprints/Interaction/BPI_Interactable.GetPromptText` _hitactor))
          (set `TextBlock.Text` _prompt (`/Game/Puzzle/UI/WBP_InteractPrompt.PromptLabel` (`self.PromptWidget`)))
          (`Widget.SetVisibility` (`self.PromptWidget`) "Visible"))
        (:`Is Not Valid`
          (`Widget.SetVisibility` (`self.PromptWidget`) "Hidden"))))))

(event `EnhancedInput|/Game/Input/IA_Interact`
  (params (ActionValue :type Boolean) (ElapsedSeconds :type "Float (double-precision)") (TriggeredSeconds :type "Float (double-precision)") (InputAction :type "InputAction Object Reference" :default "/Game/Input/IA_Interact.IA_Interact"))
  (:`Started`
    (bind _hitactor (`self.GetLookedAtInteractable`))
    (`/Engine/EditorBlueprintResources/StandardMacros.IsValid` _hitactor
      (:`Is Valid`
        (message `/Game/Puzzle/Blueprints/Interaction/BPI_Interactable.Interact` _hitactor (`self.GetOwner`))))))

(fn `GetLookedAtInteractable`
  (returns (HitActor :type "Actor Object Reference"))
  (locals (TraceStart :type "Vector Structure") (TraceEnd :type "Vector Structure"))
  (bind _asbp_third_person_character (cast `/Game/ThirdPerson/Blueprints/BP_ThirdPersonCharacter` (`self.GetOwner`)))
  (bind _followcamera (`/Game/ThirdPerson/Blueprints/BP_ThirdPersonCharacter.FollowCamera` _asbp_third_person_character))
  (bind _returnvalue (`SceneComponent.GetForwardVector` _followcamera))
  (set `local.TraceStart` (+ (`SceneComponent.K2_GetComponentLocation` _followcamera) (* _returnvalue (+ (`SpringArmComponent.TargetArmLength` (`/Game/ThirdPerson/Blueprints/BP_ThirdPersonCharacter.CameraBoom` _asbp_third_person_character)) 50.0))))
  (set `local.TraceEnd` (+ (* _returnvalue 200.0) (`local.TraceStart`)))
  (bind (_outhit _returnvalue_2) (`KismetSystemLibrary.SphereTraceSingle` (`local.TraceStart`) (`local.TraceEnd`) 15.0 "TraceTypeQuery1"))
  (if _returnvalue_2
    (bind (_bblockinghit _binitialoverlap _time _distance _location _impactpoint _normal _impactnormal _physmat _hitactor) (`GameplayStatics.BreakHitResult` _outhit))
    (if (`KismetSystemLibrary.DoesImplementInterface` _hitactor "/Game/Puzzle/Blueprints/Interaction/BPI_Interactable.BPI_Interactable_C")
      (return _hitactor)
      (else
        (return null)))
    (else
      (return null))))