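; BP_MaleNPC is an AI-controlled NPC that tracks whether it has seen BP_Boby, based purely on distance.
; Every Tick it looks up BP_Boby and writes the hasSeenBoby Blackboard flag through its AI Controller.
; Separate enter and exit radii add hysteresis: the flag sets when Boby comes close and clears only once Boby moves farther away.
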(event `self.ReceiveTick`
  (params (DeltaSeconds :type "Float (single-precision)"))
  (bind _returnvalue (`AIBlueprintHelperLibrary.GetBlackboard` (`AIBlueprintHelperLibrary.GetAIController` self)))
  (bind _returnvalue_2 (`GameplayStatics.GetActorOfClass` "/Game/AI/BP_Boby.BP_Boby_C"))
  (`/Engine/EditorBlueprintResources/StandardMacros.IsValid` _returnvalue_2
    (:`Is Valid`
      (if (`BlackboardComponent.GetValueAsBool` _returnvalue "hasSeenBoby")
        (bind _returnvalue_3 (`self.GetDistanceTo` _returnvalue_2 self))
        (if (> _returnvalue_3 1500.0)
          (`BlackboardComponent.SetValueAsBool` _returnvalue "hasSeenBoby" false))
        (elif (< _returnvalue_3 1000.0)
          (`BlackboardComponent.SetValueAsBool` _returnvalue "hasSeenBoby" true))))))

(fn `UserConstructionScript`)