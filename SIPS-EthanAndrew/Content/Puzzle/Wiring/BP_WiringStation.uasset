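; Interactable wiring station that breaks and offers a repair minigame.
; WiringEnable marks it broken and starts a timer that alerts all Wiring_neglect actors on expiry; nothing here clears either.
; Interact, regardless of broken state, opens WBP_WiringBoard in UI-only input and flags the player's interactor as in-minigame.
; Board events drive the rest: solving prints a message and closes the board after a delay, and closing restores game input.
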(event `/Game/Puzzle/Wiring/wiring_enable.wiring_enable`
  (set `self.broken` true)
  (`KismetSystemLibrary.K2_SetTimerDelegate` (delegate `wiring neglected`) 15.0))

(event `wiring neglected`
  (bind _outactors (`GameplayStatics.GetAllActorsWithInterface` "/Game/Puzzle/Wiring/wiring_neglect.wiring_neglect_C"))
  (message `/Game/Puzzle/Wiring/wiring_neglect.wiring_neglect` _outactors)
  (`KismetSystemLibrary.PrintString` "Warning: power fluctuations compromising bunker systems"))

(event `/Game/Puzzle/Blueprints/Interaction/BPI_Interactable.Interact`
  (params (Interactor :type "Actor Object Reference"))
  (bind _sips_controller (`self.sips_controller`))
  (bind _assips_player (cast `/Game/AndrewImports/Blueprints/SIPS_Player` (`GameplayStatics.GetPlayerPawn` 0)))
  (bind _output_get (set `self.sips_character` _assips_player))
  (set `self.sips_controller` (`GameplayStatics.GetPlayerController` 0))
  (set `/Game/Puzzle/Blueprints/Interaction/BPC_Interactor.bInMinigame` true (`self.GetComponentByClass` _output_get "/Game/Puzzle/Blueprints/Interaction/BPC_Interactor.BPC_Interactor_C"))
  (bind _returnvalue (`|CreateWidget` "/Game/Puzzle/Wiring/WBP_WiringBoard.WBP_WiringBoard_C" (`self.sips_controller`)))
  (`|ExecutionSequence`
    (:`then_0`
      (`UserWidget.AddToViewport` _returnvalue 0))
    (:`then_1`
      (add `/Game/Puzzle/Wiring/WBP_WiringBoard.OnBoardClosed` _returnvalue (delegate `HandleBoardClosed`))
      (`WidgetBlueprintLibrary.SetInputMode_UIOnlyEx` _sips_controller _returnvalue))
    (:`then_2`
      (set `PlayerController.bShowMouseCursor` true _sips_controller))
    (:`then_3`
      (set `self.BoardWidget` _returnvalue)
      (add `/Game/Puzzle/Wiring/WBP_WiringBoard.OnBoardSolved` _returnvalue (delegate `HandleBoardSolved`)))))

(event `HandleBoardClosed`
  (bind _sips_controller (`self.sips_controller`))
  (`|ExecutionSequence`
    (:`then_0`
      (`WidgetBlueprintLibrary.SetInputMode_GameOnly` _sips_controller))
    (:`then_1`
      (set `PlayerController.bShowMouseCursor` false _sips_controller)
      (set `/Game/Puzzle/Blueprints/Interaction/BPC_Interactor.bInMinigame` false (`self.GetComponentByClass` (`self.sips_character`) "/Game/Puzzle/Blueprints/Interaction/BPC_Interactor.BPC_Interactor_C")))))

(event `HandleBoardSolved`
  (bind _boardwidget (`self.BoardWidget`))
  (`KismetSystemLibrary.PrintString` "Life support restored!")
  (`KismetSystemLibrary.Delay` 1.5)
  (`/Engine/EditorBlueprintResources/StandardMacros.IsValid` _boardwidget
    (:`Is Valid`
      (`/Game/Puzzle/Wiring/WBP_WiringBoard.CloseBoard` _boardwidget))))

(fn `GetPromptText`
  (returns (Prompt :type Text))
  (if (`self.broken`)
    (return "Press E to repair wiring")
    (else
      (return "System functional"))))

(fn `UserConstructionScript`)