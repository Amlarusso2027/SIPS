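; Player character Blueprint that handles movement, horizontal mouse turning and a sprint that costs Hunger.
; Forward and lateral axes move along the capsule's vectors, while the Run input switches walk speed through SprintStart and SprintStop.
; Sprinting starts HungerDrain, a self-calling Delay loop that decrements Hunger each second and ends the sprint at zero.
; BeginPlay adds the Hunger widget to the viewport.
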(event `HungerDrain`
  (bind _output_get (set `self.Hunger` (`KismetMathLibrary.Clamp` (- (`self.Hunger`) 1) 0 (`self.MaxHunger`))))
  (if (== _output_get 0)
    (`self.SprintStop`)
    (elif (`self.IsRunning`)
      (`KismetSystemLibrary.Delay` 1.0)
      (`self.HungerDrain`))))

(event `InputAction|Run`
  (params (Key :type "Key Structure"))
  ; Movement
  (:`Pressed`
    (`self.SprintStart`))
  (:`Released`
    (`self.SprintStop`)))

(event `InputAxis|Turn`
  (params (AxisValue :type "Float (single-precision)"))
  ; Camera-Mouse
  (`self.AddControllerYawInput` AxisValue))

(event `self.ReceiveBeginPlay`
  (bind _returnvalue (`|CreateWidget` "/Game/AndrewImports/Blueprints/Hunger.Hunger_C"))
  (`UserWidget.AddToViewport` _returnvalue 0))

(event `InputAxis|Forward`
  (params (AxisValue :type "Float (single-precision)"))
  ; Movement
  (`self.AddMovementInput` (`SceneComponent.GetForwardVector` (`self.CapsuleComponent`)) AxisValue))

(event `self.ReceiveActorBeginOverlap`
  (params (OtherActor :type "Actor Object Reference")))

(event `InputAxis|Lateral`
  (params (AxisValue :type "Float (single-precision)"))
  (`self.AddMovementInput` (`SceneComponent.GetRightVector` (`self.CapsuleComponent`)) AxisValue))

(fn `SprintStart`
  (set `CharacterMovementComponent.MaxWalkSpeed` 600.0 (`self.CharacterMovement`))
  (set `self.IsRunning` true)
  (`self.HungerDrain`))

(fn `SprintStop`
  (set `CharacterMovementComponent.MaxWalkSpeed` 150.0 (`self.CharacterMovement`))
  (set `self.IsRunning` false))

(fn `UserConstructionScript`)